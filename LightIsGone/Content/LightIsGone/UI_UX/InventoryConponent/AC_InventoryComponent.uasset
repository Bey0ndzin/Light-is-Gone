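; AC_InventoryComponent is an inventory component that shows and hides the inventory UI for the local player.
; ShowInventory checks that player controller 0 is local, then creates a new WB_Inventory widget, stores it and adds it to the viewport.
; HideInventory removes the stored widget from the viewport if it is still valid.
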(fn ShowInventory
  (bind _returnvalue (Game|GetPlayerController 0))
  (if (Pawn|IsLocalPlayerController _returnvalue)
    (bind _returnvalue_2 (UserInterface|CreateWidget "/Game/LightIsGone/UI_UX/InventoryConponent/WB_Inventory.WB_Inventory_C" _returnvalue))
    (bind _output_get (Variables|Default|SetWB_Inventory _returnvalue_2))
    (UserInterface|Viewport|AddtoViewport _output_get 0)))

(fn HideInventory
  (Utilities|IsValid (Variables|Default|GetWB_Inventory)
    (:Is%20Valid
      (Widget|RemovefromParent (Variables|Default|GetWB_Inventory)))))
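; AC_OptionsComponent is a component that switches the local player between the HUD and the options menu.
; ShowOptions removes the HUD, creates WB_Options for player controller 0 and shows the mouse cursor; HideOptions removes the menu, calls ShowHUD and hides the cursor.
; Both widgets are created anew each time they are shown rather than reused, and creation only runs on a local player controller.
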(fn ShowOptions
  (bind _returnvalue (Game|GetPlayerController 0))
  (CallFunction|HideHUD)
  (if (Pawn|IsLocalPlayerController _returnvalue)
    (bind _returnvalue_2 (UserInterface|CreateWidget "/Game/LightIsGone/UI_UX/InventoryConponent/WB_Options.WB_Options_C" _returnvalue))
    (bind _output_get (Variables|Default|SetWB_Options _returnvalue_2))
    (UserInterface|Viewport|AddtoViewport _output_get 0)
    (Variables|/Script/Engine.PlayerController|SetbShowMouseCursor _returnvalue true)))

(fn HideOptions
  (Utilities|IsValid (Variables|Default|GetWB_Options)
    (:Is%20Valid
      (Widget|RemovefromParent (Variables|Default|GetWB_Options))
      (CallFunction|ShowHUD)
      (Variables|/Script/Engine.PlayerController|SetbShowMouseCursor (Game|GetPlayerController 0) false))))

(fn HideHUD
  (Utilities|IsValid (Variables|Default|GetWB_HUD)
    (:Is%20Valid
      (Widget|RemovefromParent (Variables|Default|GetWB_HUD)))))

(fn ShowHUD
  (bind _returnvalue (Game|GetPlayerController 0))
  (if (Pawn|IsLocalPlayerController _returnvalue)
    (bind _returnvalue_2 (UserInterface|CreateWidget "/Game/LightIsGone/UI_UX/WB_HUD.WB_HUD_C" _returnvalue))
    (bind _output_get (Variables|Default|SetWB_HUD _returnvalue_2))
    (UserInterface|Viewport|AddtoViewport _output_get 0)))